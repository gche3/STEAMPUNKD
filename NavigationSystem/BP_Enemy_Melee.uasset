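; Melee enemy that wanders the navmesh until PawnSensing spots the third-person player, then chases them with AI MoveTo.
; Tick switches between chase and timed random roaming via DoOnce gates; a retriggerable delay clears the seen flag shortly after sight is lost.
; Body contact damages the player and destroys the enemy with an emitter; its knockback launch is multiplied by zero.
; Touching the back weak spot instead awards score and destroys it.
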(event OnSeePawn(PawnSensing)
  (params (Pawn :type Pawn%20Object%20Reference))
  (bind _asbp_third_person_character (Utilities|Casting|CastToBP_ThirdPersonCharacter Pawn))
  (Variables|Default|SetPlayerFollowed _asbp_third_person_character)
  (Utilities|FlowControl|Sequence
    (:then_0
      (Variables|Default|SetSeenPlayer true))
    (:then_1
      (Utilities|FlowControl|RetriggerableDelay 0.6)
      (Variables|Default|SetSeenPlayer false))))

(event OnComponentBeginOverlap(weakness_back)
  (params (OverlappedComponent :type Primitive%20Component%20Object%20Reference) (OtherActor :type Actor%20Object%20Reference) (OtherComp :type Primitive%20Component%20Object%20Reference) (OtherBodyIndex :type Integer) (bFromSweep :type Boolean) (SweepResult :type Hit%20Result%20Structure%20%28by%20ref%29))
  (bind _asbp_third_person_character (Utilities|Casting|CastToBP_ThirdPersonCharacter OtherActor))
  (Variables|/Game/ThirdPerson/Blueprints/BP_ThirdPersonCharacter.BP_ThirdPersonCharacter_C|SetScore _asbp_third_person_character (Math|Conversions|ToFloat(Integer) (+ (Variables|/Game/ThirdPerson/Blueprints/BP_ThirdPersonCharacter.BP_ThirdPersonCharacter_C|GetScore _asbp_third_person_character) 20)))
  (Effects|SpawnEmitteratLocation 0 (Transformation|GetActorLocation))
  (Actor|DestroyActor))

(event OnComponentBeginOverlap(Body_0)
  (params (OverlappedComponent :type Primitive%20Component%20Object%20Reference) (OtherActor :type Actor%20Object%20Reference) (OtherComp :type Primitive%20Component%20Object%20Reference) (OtherBodyIndex :type Integer) (bFromSweep :type Boolean) (SweepResult :type Hit%20Result%20Structure%20%28by%20ref%29))
  (bind _asbp_third_person_character (Utilities|Casting|CastToBP_ThirdPersonCharacter OtherActor))
  (Character|LaunchCharacter _asbp_third_person_character (* (Math|Vector|MakeVector (.x (Math|Vector|Normalize (Math|Vector|MakeVector (.x (Math|Vector|GetUnitDirection(Vector) (Transformation|GetWorldLocation (Variables|Collision|GetCapsuleComponent)) (Transformation|GetActorLocation _asbp_third_person_character))) (.y (Math|Vector|GetUnitDirection(Vector) (Transformation|GetWorldLocation (Variables|Collision|GetCapsuleComponent)) (Transformation|GetActorLocation _asbp_third_person_character))) 0.0))) (.y (Math|Vector|Normalize (Math|Vector|MakeVector (.x (Math|Vector|GetUnitDirection(Vector) (Transformation|GetWorldLocation (Variables|Collision|GetCapsuleComponent)) (Transformation|GetActorLocation _asbp_third_person_character))) (.y (Math|Vector|GetUnitDirection(Vector) (Transformation|GetWorldLocation (Variables|Collision|GetCapsuleComponent)) (Transformation|GetActorLocation _asbp_third_person_character))) 0.0))) 0.5) "") false false)
  (Game|Damage|ApplyDamage _asbp_third_person_character 5e+01 0 0)
  (Effects|SpawnEmitteratLocation 0 (Transformation|GetActorLocation))
  (Actor|DestroyActor))

(event Custom|MoveNPC
  (bind _output_get (Variables|Default|SetRandom%20Location (.RandomLocation (AI|Navigation|GetRandomReachablePointinRadius (Transformation|GetActorLocation) 1e+03 0 0))))
  (AI|AIMoveTo self _output_get 0 5.0 false))

(event EventTick
  (params (DeltaSeconds :type Float%20%28single-precision%29))
  (if (Variables|Default|GetSeenPlayer)
    (Utilities|FlowControl|DoOnce false :!label _label
      (:Completed
        (AI|AIMoveTo self (Transformation|GetActorLocation (Variables|Default|GetPlayerFollowed)) 0 5.0 false
          (:then
            (goto _label Reset)))))
    (else
      (Utilities|FlowControl|DoOnce false :!label _label_2
        (:Completed
          (CallFunction|MoveNPC)
          (Utilities|FlowControl|Delay 4.0)
          (goto _label_2 Reset))))))

(fn ConstructionScript)

(fn ChasePlayer)