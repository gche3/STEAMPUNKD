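; BP_bomb is a contact bomb that explodes, knocks back and damages the first-person player.
; On overlap with BP_FirstPersonCharacter, it spawns P_Explosion at the bomb and applies fixed damage before destroying itself.
; The launch direction is flattened away from the bomb, given a fixed upward component and scaled by LaunchV.
; Any other overlap destroys the bomb and spawns the explosion without setting its location.
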(event OnComponentBeginOverlap(round_bomb)
  (params (OverlappedComponent :type Primitive%20Component%20Object%20Reference) (OtherActor :type Actor%20Object%20Reference) (OtherComp :type Primitive%20Component%20Object%20Reference) (OtherBodyIndex :type Integer) (bFromSweep :type Boolean) (SweepResult :type Hit%20Result%20Structure%20%28by%20ref%29))
  (bind _asbp_first_person_character (Utilities|Casting|CastToBP_FirstPersonCharacter OtherActor)
    (:then
      (Effects|SpawnEmitteratLocation "/Game/StarterContent/Particles/P_Explosion.P_Explosion" (Transformation|GetWorldLocation (Variables|Default|Getround_bomb)))
      (Character|LaunchCharacter _asbp_first_person_character (* (Math|Vector|MakeVector (.x (Math|Vector|Normalize (Math|Vector|MakeVector (.x (Math|Vector|GetUnitDirection(Vector) (Transformation|GetWorldLocation (Variables|Default|Getround_bomb)) (Transformation|GetActorLocation _asbp_first_person_character))) (.y (Math|Vector|GetUnitDirection(Vector) (Transformation|GetWorldLocation (Variables|Default|Getround_bomb)) (Transformation|GetActorLocation _asbp_first_person_character))) 0.0))) (.y (Math|Vector|Normalize (Math|Vector|MakeVector (.x (Math|Vector|GetUnitDirection(Vector) (Transformation|GetWorldLocation (Variables|Default|Getround_bomb)) (Transformation|GetActorLocation _asbp_first_person_character))) (.y (Math|Vector|GetUnitDirection(Vector) (Transformation|GetWorldLocation (Variables|Default|Getround_bomb)) (Transformation|GetActorLocation _asbp_first_person_character))) 0.0))) 0.5) (Variables|Default|GetLaunch%20V)) false false)
      (Game|Damage|ApplyDamage _asbp_first_person_character 2e+01 0 0)
      (Actor|DestroyActor))
    (:CastFailed
      (Actor|DestroyActor)
      (Effects|SpawnEmitteratLocation "/Game/StarterContent/Particles/P_Explosion.P_Explosion" "0, 0, 0"))))

(fn ConstructionScript)