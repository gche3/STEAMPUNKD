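; BP_Bullet is a projectile actor that damages and knocks back the first-person player character on contact.
; When its static mesh overlaps that character, it spawns an explosion effect and sound, applies fixed damage, then destroys itself.
; The knockback launches the character along the flattened, normalized bullet-to-character direction with a fixed upward component, scaled by LaunchV.
; Overlapping any other actor simply destroys the bullet.
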(event OnComponentBeginOverlap(StaticMesh)
  (params (OverlappedComponent :type Primitive%20Component%20Object%20Reference) (OtherActor :type Actor%20Object%20Reference) (OtherComp :type Primitive%20Component%20Object%20Reference) (OtherBodyIndex :type Integer) (bFromSweep :type Boolean) (SweepResult :type Hit%20Result%20Structure%20%28by%20ref%29))
  (bind _staticmesh (Variables|Default|GetStaticMesh))
  (bind _returnvalue (Transformation|GetWorldLocation _staticmesh))
  (bind _asbp_first_person_character (Utilities|Casting|CastToBP_FirstPersonCharacter OtherActor)
    (:then
      (Effects|SpawnEmitteratLocation "/Game/StarterContent/Particles/P_Explosion.P_Explosion" _returnvalue)
      (Audio|PlaySoundatLocation "/Game/FPWeapon/Audio/mixkit-game-gun-shot-1662.mixkit-game-gun-shot-1662" _returnvalue "0, 0, 0" 1.0 1.0 0.0 0 0 0 0)
      (Character|LaunchCharacter _asbp_first_person_character (* (Math|Vector|MakeVector (.x (Math|Vector|Normalize (Math|Vector|MakeVector (.x (Math|Vector|GetUnitDirection(Vector) (Transformation|GetWorldLocation (Variables|Default|GetStaticMesh)) (Transformation|GetActorLocation _asbp_first_person_character))) (.y (Math|Vector|GetUnitDirection(Vector) (Transformation|GetWorldLocation (Variables|Default|GetStaticMesh)) (Transformation|GetActorLocation _asbp_first_person_character))) 0.0))) (.y (Math|Vector|Normalize (Math|Vector|MakeVector (.x (Math|Vector|GetUnitDirection(Vector) (Transformation|GetWorldLocation (Variables|Default|GetStaticMesh)) (Transformation|GetActorLocation _asbp_first_person_character))) (.y (Math|Vector|GetUnitDirection(Vector) (Transformation|GetWorldLocation (Variables|Default|GetStaticMesh)) (Transformation|GetActorLocation _asbp_first_person_character))) 0.0))) 0.5) (Variables|Default|GetLaunch%20V)) false false)
      (Game|Damage|ApplyDamage _asbp_first_person_character 1e+01 0 0)
      (Actor|DestroyActor))
    (:CastFailed
      (Actor|DestroyActor))))

(fn ConstructionScript)